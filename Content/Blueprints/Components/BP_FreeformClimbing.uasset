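; Character component for freeform climbing, toggled by input and started when a forward line trace hits a climbable physical material.
; Climbing switches to Flying movement and a climbing input context, with movement input following the surface's up and right axes.
; Each tick re-traces to face the wall; when the wall is lost, a downward sphere trace finds a ledge to mantle or climbing stops.
; Mantling, also triggerable by input, plays a montage while moving the root component onto the ledge.
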(event Custom|ClimbToLedge
  (params (LedgeLocation :type Vector))
  (bind _returnvalue (Components|GetOwner))
  (bind _rootcomponent (Variables|/Script/Engine.Actor|GetRootComponent _returnvalue))
  (bind _ascharacter (Utilities|Casting|CastToCharacter _returnvalue))
  (Variables|Default|SetIsClimbing false)
  (bind _returnvalue_2 (Animation|Montage|MontagePlay (Components|SkeletalMesh|GetAnimInstance (Variables|/Script/Engine.Character|GetMesh _ascharacter)) "/Game/Animations/mantle_up_Montage.mantle_up_Montage" 1.0 "MontageLength" 0.0 true))
  (Components|MoveComponentTo _rootcomponent LedgeLocation (Variables|/Script/Engine.SceneComponent|GetRelativeRotation _rootcomponent) false false _returnvalue_2 false)
  (CallFunction|StopClimbing))

(event Input|EnhancedActionEvents|EnhancedInputActionIA_Climb
  (params (ActionValue :type Boolean) (ElapsedSeconds :type Float%20%28double-precision%29) (TriggeredSeconds :type Float%20%28double-precision%29) (InputAction :type Input%20Action%20Object%20Reference :default "/Game/ThirdPerson/Input/Actions/IA_Climb.IA_Climb"))
  (bind _player_controller (Variables|Components|GetPlayer%20Controller))
  (bind _returnvalue (PlayerController|LocalPlayerSubsystems|GetEnhancedInputLocalPlayerSubsystem _player_controller))
  (if (Variables|Default|GetIsClimbing)
    (CallFunction|StopClimbing)
    (else
      (bind _didstartclimbing (CallFunction|StartClimbing))
      (if _didstartclimbing
        (Input|RemoveMappingContext _returnvalue "/Game/ThirdPerson/Input/IMC_Default.IMC_Default" "(bIgnoreAllPressedKeysUntilRelease=True,bForceImmediately=False,bNotifyUserSettings=False)")
        (Input|AddMappingContext _returnvalue "/Game/ThirdPerson/Input/IMC_Climbing.IMC_Climbing" 0 "(bIgnoreAllPressedKeysUntilRelease=True,bForceImmediately=False,bNotifyUserSettings=False)")
        (bind _ascharacter (Utilities|Casting|CastToCharacter (Components|GetOwner)))
        (bind _returnvalue_2 (Animation|Montage|MontagePlay (Components|SkeletalMesh|GetAnimInstance (Variables|/Script/Engine.Character|GetMesh _ascharacter)) "/Game/Animations/begin_climb_montage.begin_climb_montage" 1.0 "MontageLength" 0.0 true))
        (Utilities|FlowControl|Delay _returnvalue_2)
        (Variables|Default|SetIsClimbing true)))))

(event Input|EnhancedActionEvents|EnhancedInputActionIA_ClimbMove
  (params (ActionValue :type Vector%202D%20Structure) (ElapsedSeconds :type Float%20%28double-precision%29) (TriggeredSeconds :type Float%20%28double-precision%29) (InputAction :type Input%20Action%20Object%20Reference :default "/Game/ThirdPerson/Input/Actions/IA_ClimbMove.IA_ClimbMove"))
  (bind _surfacenormal (Variables|Default|GetSurfaceNormal))
  (bind _player_controller (Variables|Components|GetPlayer%20Controller))
  (bind _returnvalue (Pawn|GetControlledPawn _player_controller))
  (bind _returnvalue_2 (Math|Rotator|MakeRotfromX _surfacenormal))
  (Pawn|Input|AddMovementInput _returnvalue (Math|Vector|GetUpVector _returnvalue_2) (.y ActionValue) false)
  (Pawn|Input|AddMovementInput _returnvalue (Math|Vector|GetRightVector _returnvalue_2) (.x ActionValue) false))

(event Input|EnhancedActionEvents|EnhancedInputActionIA_Mantle
  (params (ActionValue :type Boolean) (ElapsedSeconds :type Float%20%28double-precision%29) (TriggeredSeconds :type Float%20%28double-precision%29) (InputAction :type Input%20Action%20Object%20Reference :default "/Game/ThirdPerson/Input/Actions/IA_Mantle.IA_Mantle"))
  (bind (_ledgefound _ledgelocation) (CallFunction|PeakTrace))
  (if _ledgefound
    (CallFunction|ClimbtoLedge _ledgelocation)))

(event EventBeginPlay
  (bind _ascharacter (Utilities|Casting|CastToCharacter (Components|GetOwner)))
  (Variables|Default|SetCharacter%20Movement (Variables|/Script/Engine.Character|GetCharacterMovement _ascharacter))
  (bind _asplayer_controller (Utilities|Casting|CastToPlayerController (Pawn|GetController _ascharacter)))
  (Variables|Components|SetPlayer%20Controller _asplayer_controller))

(event EventTick
  (params (DeltaSeconds :type Float%20%28single-precision%29))
  (if (Variables|Default|GetIsClimbing)
    (bind (_returnvalue _outhit) (CallFunction|ClimbingTrace))
    (if _returnvalue
      (Variables|Default|SetSurfaceNormal (Math|Vector|NegateVector (.ImpactNormal (Collision|BreakHitResult _outhit))))
      (Transformation|SetActorRotation (Components|GetOwner) (Math|Rotator|MakeRotfromX (Math|Vector|NegateVector (.ImpactNormal (Collision|BreakHitResult _outhit)))))
      (else
        (bind (_ledgefound _ledgelocation) (CallFunction|PeakTrace))
        (if _ledgefound
          (CallFunction|ClimbtoLedge _ledgelocation)
          (else
            (CallFunction|StopClimbing)))))))

(fn StartClimbing
  (bind _returnvalue (Components|GetOwner))
  (bind (_returnvalue_2 _outhit) (CallFunction|ClimbingTrace))
  (if (and _returnvalue_2 (== (.PhysMat (Collision|BreakHitResult _outhit)) "/Game/PhysMaterials/Climbable_PM.Climbable_PM"))
    (Variables|Default|SetIsClimbing true)
    (Transformation|SetActorLocationAndRotation _returnvalue (+ (.Location (Collision|BreakHitResult _outhit)) (* (.ImpactNormal (Collision|BreakHitResult _outhit)) 5e+01)) (Math|Rotator|MakeRotfromX (Math|Vector|NegateVector (.ImpactNormal (Collision|BreakHitResult _outhit)))))
    (bind _ascharacter (Utilities|Casting|CastToCharacter _returnvalue))
    (Pawn|Components|CharacterMovement|SetMovementMode (Variables|/Script/Engine.Character|GetCharacterMovement _ascharacter) "MOVE_Flying" 0)
    (return true)
    (else
      (return false))))

(fn ClimbingTrace
  (bind _returnvalue (Components|GetOwner))
  (bind _traceheightoffset (Variables|Default|GetTraceHeightOffset))
  (bind _returnvalue_2 (Transformation|GetActorLocation _returnvalue))
  (bind _returnvalue_3 (Transformation|GetActorUpVector _returnvalue))
  (bind _returnvalue_4 (* _traceheightoffset _returnvalue_3))
  (bind _returnvalue_5 (+ _returnvalue_4 _returnvalue_2))
  (bind (_outhit _returnvalue_6) (Collision|LineTraceByChannel _returnvalue_5 (+ _returnvalue_5 (* (Transformation|GetActorForwardVector _returnvalue) (Variables|Default|GetBeginClimbTraceDistance))) "TraceTypeQuery1" false 0 "ForDuration"))
  (return _returnvalue_6 _outhit))

(fn StopClimbing
  (bind _player_controller (Variables|Components|GetPlayer%20Controller))
  (bind _returnvalue (PlayerController|LocalPlayerSubsystems|GetEnhancedInputLocalPlayerSubsystem _player_controller))
  (Input|RemoveMappingContext _returnvalue "/Game/ThirdPerson/Input/IMC_Climbing.IMC_Climbing" "(bIgnoreAllPressedKeysUntilRelease=True,bForceImmediately=False,bNotifyUserSettings=False)")
  (Input|AddMappingContext _returnvalue "/Game/ThirdPerson/Input/IMC_Default.IMC_Default" 0 "(bIgnoreAllPressedKeysUntilRelease=True,bForceImmediately=False,bNotifyUserSettings=False)")
  (Pawn|Components|CharacterMovement|SetMovementMode (Variables|Default|GetCharacter%20Movement) "MOVE_Falling" 0)
  (Variables|Default|SetIsClimbing false))

(fn PeakTrace
  (bind _returnvalue (Components|GetOwner))
  (bind _returnvalue_2 (Transformation|GetActorLocation _returnvalue))
  (bind _returnvalue_3 (Transformation|GetActorForwardVector _returnvalue))
  (bind _returnvalue_4 (* _returnvalue_3 1e+02))
  (bind _returnvalue_5 (+ _returnvalue_2 _returnvalue_4))
  (bind (_outhit _returnvalue_6) (Collision|SphereTraceByChannel (Math|Vector|MakeVector (.x _returnvalue_5) (.y _returnvalue_5) (+ (.z _returnvalue_5) 1e+02)) (Math|Vector|MakeVector (.x _returnvalue_5) (.y _returnvalue_5) (- (.z _returnvalue_5) 2e+01)) 2e+01 "TraceTypeQuery3" false 0 "None"))
  (if _returnvalue_6
    (return true (+ "0.000000,0.000000,90.000000" (.Location (Collision|BreakHitResult _outhit))))
    (else
      (return false "0, 0, 0"))))