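; Shard inventory component for BP_ThirdPersonCharacter that keeps track of the shards collected.
; On BeginPlay it casts its owner to that character and binds an event to the character's ShardCollected dispatcher.
; CollectShard adds a shard to the Shards array without duplicates and prints the running count as debug text.
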(event Custom|CollectShard
  (params (Shard :type BP%20Shard%20Collectable%20Object%20Reference))
  (bind _shards (Variables|Default|GetShards))
  (Utilities|Array|AddUnique _shards Shard)
  (Development|PrintString (Utilities|String|Append (Utilities|String|ToString(Integer) (Utilities|Array|Length _shards)) " shards collected")))

(event EventBeginPlay
  (bind _asbp_third_person_character (Utilities|Casting|CastToBP_ThirdPersonCharacter (Components|GetOwner)))
  (EventDispatchers|BindEventtoShardCollected _asbp_third_person_character (EventDispatchers|CreateEvent :!event Custom|CollectShard)))