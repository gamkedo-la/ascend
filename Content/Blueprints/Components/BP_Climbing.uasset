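; Climbing component that lets its owning Character grab a ledge when C is pressed.
; Every tick, debug-drawn sphere traces store a wall point and normal ahead and a height point from a vertical sweep.
; If both points are non-zero, C disables movement and moves the root to hang below the height point, facing the wall.
; The parent shape's overlaps set IsNearLedge, which does not yet gate anything.
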(event Custom|OnComponentBeginOverlap
  (params (OverlappedComponent :type Primitive%20Component%20Object%20Reference) (OtherActor :type Actor%20Object%20Reference) (OtherComp :type Primitive%20Component%20Object%20Reference) (OtherBodyIndex :type Integer) (bFromSweep :type Boolean) (SweepResult :type Hit%20Result%20Structure%20%28by%20ref%29))
  (Variables|Default|SetbIsNearLedge true))

(event Custom|OnComponentEndOverlap
  (params (OverlappedComponent :type Primitive%20Component%20Object%20Reference) (OtherActor :type Actor%20Object%20Reference) (OtherComp :type Primitive%20Component%20Object%20Reference) (OtherBodyIndex :type Integer))
  (Variables|Default|SetbIsNearLedge false))

(event EventBeginPlay
  (Collision|AssignOnComponentBeginOverlap (Variables|Default|GetCollider) (EventDispatchers|CreateEvent :!event Custom|OnComponentBeginOverlap))
  (Collision|BindEventtoOnComponentEndOverlap (Variables|Default|GetCollider) (EventDispatchers|CreateEvent :!event Custom|OnComponentEndOverlap))
  (bind _ascharacter (Utilities|Casting|CastToCharacter (Components|GetOwner))
    (:then
      (Variables|Default|SetMovementComponent (Variables|/Script/Engine.Character|GetCharacterMovement _ascharacter)))
    (:CastFailed
      (Development|PrintString "BP_Climbing owning actor is not a character")))
  (bind _asshape_component (Utilities|Casting|CastToShapeComponent (Transformation|GetAttachParent))
    (:then
      (Variables|Default|SetCollider _asshape_component))
    (:CastFailed
      (Development|PrintString "BP_Climbing Attach parent is not a shape component"))))

(event EventTick
  (params (DeltaSeconds :type Float%20%28single-precision%29))
  (if (Variables|Default|GetbIsNearLedge)
    _
    (else
      _))
  (Utilities|FlowControl|Sequence
    (:then_0
      (CallFunction|HeightTrace))
    (:then_1
      (CallFunction|ForwardTrace 0.0 1.5e+02 2e+01))))

(event Input|KeyboardEvents|C
  (params (Key :type Key%20Structure :default "None"))
  (bind _walllocation (Variables|Default|GetWallLocation))
  (bind _wallnormal (Variables|Default|GetWallNormal))
  (bind _wallnormal_2 (Variables|Default|GetWallNormal))
  (bind _returnvalue (Math|Conversions|RotationFromXVector _wallnormal_2))
  (bind _returnvalue_2 (* _wallnormal 22.0))
  (:Pressed
    (if (CallFunction|HasGrabTarget)
      (Pawn|Components|CharacterMovement|DisableMovement (Variables|Default|GetMovementComponent))
      (Variables|Default|SetbIsClimbing true)
      (Components|MoveComponentTo (Variables|/Script/Engine.Actor|GetRootComponent (Components|GetOwner)) (Math|Vector|MakeVector (+ (.x _returnvalue_2) (.x _walllocation)) (+ (.y _returnvalue_2) (.y _walllocation)) (- (.z (Variables|Default|GetHeightLocation)) 45.0)) (Math|Rotator|MakeRotator (.roll _returnvalue) (.pitch _returnvalue) (- (.yaw _returnvalue) 1.8e+02)) false false 0.2 false)
      (Components|Movement|StopMovementImmediately (Variables|Default|GetMovementComponent)))))

(fn ForwardTrace
  (params (Vertical%20Offset :type Float%20%28double-precision%29) (Trace%20Distance :type Float%20%28double-precision%29) (Radius :type Float%20%28double-precision%29))
  (bind _returnvalue (Components|GetOwner))
  (bind _returnvalue_2 (Transformation|GetActorLocation _returnvalue))
  (bind _returnvalue_3 (Transformation|GetActorForwardVector _returnvalue))
  (bind (_x _y _z) (Math|Vector|BreakVector _returnvalue_3))
  (bind (_x_2 _y_2 _z_2) (Math|Vector|BreakVector _returnvalue_2))
  (bind _returnvalue_4 (- _z_2 Vertical%20Offset))
  (bind _returnvalue_5 (Math|Vector|MakeVector _x_2 _y_2 _returnvalue_4))
  (bind (_outhit _returnvalue_6) (Collision|SphereTraceByChannel _returnvalue_5 (+ _returnvalue_5 (Math|Vector|MakeVector (* _x Trace%20Distance) (* _y Trace%20Distance) (- _z 0.0))) Radius "TraceTypeQuery3" false 0 "ForOneFrame"))
  (if _returnvalue_6
    (bind _output_get (Variables|Default|SetWallLocation (.Location (Collision|BreakHitResult _outhit))))
    (Development|PrintString (Utilities|String|ToString(Vector) _output_get) true true "(R=0.000000,G=0.660000,B=1.000000,A=1.000000)" 2.0 "wallloc")
    (Variables|Default|SetWallNormal (.Normal (Collision|BreakHitResult _outhit)))))

(fn HeightTrace
  (bind _returnvalue (Components|GetOwner))
  (bind _returnvalue_2 (Transformation|GetActorLocation _returnvalue))
  (bind _returnvalue_3 (Transformation|GetActorForwardVector _returnvalue))
  (bind _returnvalue_4 (* _returnvalue_3 5e+01))
  (bind _returnvalue_5 (+ _returnvalue_2 _returnvalue_4))
  (bind (_outhit _returnvalue_6) (Collision|SphereTraceByChannel (Math|Vector|MakeVector (.x _returnvalue_5) (.y _returnvalue_5) (+ (.z _returnvalue_5) 2.5e+02)) (Math|Vector|MakeVector (.x _returnvalue_5) (.y _returnvalue_5) (- (.z _returnvalue_5) 2.5e+02)) 2e+01 "TraceTypeQuery3" false 0 "ForOneFrame"))
  (if _returnvalue_6
    (bind _output_get (Variables|Default|SetHeightLocation (.Location (Collision|BreakHitResult _outhit))))
    (Development|PrintString (Utilities|String|ToString(Vector) _output_get) true true "(R=0.000000,G=0.666948,B=1.000000,A=1.000000)" 2.0 "heightloc")
    (if (Math|Float|InRange(Float) (- (.z (Transformation|GetWorldLocation (Variables|/Script/Engine.Actor|GetRootComponent (Components|GetOwner)))) (.z (Variables|Default|GetHeightLocation))) -1.5e+02 0.0)
      _)))

(fn HasGrabTarget
  (return (and (not (Math|Vector|VectorIsZero (Variables|Default|GetWallLocation))) (not (Math|Vector|VectorIsZero (Variables|Default|GetHeightLocation))))))