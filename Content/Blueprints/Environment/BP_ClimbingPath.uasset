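; BP_ClimbingPath is an environment actor that lays out a climbing path of instanced meshes on a wall along a spline.
; The construction script steps along the spline by Spacing, sphere-tracing a short distance along the actor's forward vector at each point.
; Hits get an instance at the impact point, facing along the surface normal.
; Misses print a warning, and a non-positive Spacing is rejected to avoid an endless loop.
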(event EventBeginPlay)

(event Collision|EventActorBeginOverlap
  (params (OtherActor :type Actor%20Object%20Reference)))

(event EventTick
  (params (DeltaSeconds :type Float%20%28single-precision%29)))

(fn ConstructionScript
  (CallFunction|CreateMeshInstances))

(fn CreateMeshInstances
  (if (> (Variables|Default|GetSpacing) 0.0)
    (while (<= (LocalVariables|GetDistanceAlongSpline) (Spline|GetSplineLength (Variables|Default|GetSpline)))
      (Utilities|FlowControl|Sequence
        (:then_0
          (bind (_outhit _returnvalue) (Collision|SphereTraceByChannel (Spline|GetLocationatDistanceAlongSpline (Variables|Default|GetSpline) (stale _output_get) "World") (+ (* (Transformation|GetActorForwardVector) 1e+02) (Spline|GetLocationatDistanceAlongSpline (Variables|Default|GetSpline) (stale _output_get) "World")) 5.0 "TraceTypeQuery1" false 0 "None"))
          (if _returnvalue
            (Components|InstancedStaticMesh|AddInstance (Variables|Default|GetInstancedStaticMesh) (Math|Transform|MakeTransform (.ImpactPoint (Collision|BreakHitResult _outhit)) (Math|Rotator|FindLookatRotation (.ImpactPoint (Collision|BreakHitResult _outhit)) (+ (.ImpactPoint (Collision|BreakHitResult _outhit)) (* (.ImpactNormal (Collision|BreakHitResult _outhit)) 1e+02))) "1.000000,1.000000,1.000000") true)
            (else
              (Development|PrintString "Climbing path is too far from a wall"))))
        (:then_1
          (bind _output_get (LocalVariables|SetDistanceAlongSpline (+ (LocalVariables|GetDistanceAlongSpline) (Variables|Default|GetSpacing)))))))
    (else
      (Development|PrintString "Spacing must be set highter than zero to prevent endless while loop"))))