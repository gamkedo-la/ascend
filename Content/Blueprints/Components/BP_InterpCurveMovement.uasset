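; Actor component that moves its owner back and forth along a list of control points, reversing at each end.
; Each tick it lerps between the current and target points, easing with a float curve sampled over a per-segment Duration.
; Points are world positions or offsets from the owner's starting location, which is captured on BeginPlay before snapping to the first point.
; It prints a warning when fewer than two points are set.
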(event EventBeginPlay
  (CallFunction|SetInitialPosition))

(event EventTick
  (params (DeltaSeconds :type Float%20%28single-precision%29))
  (Variables|Default|SetInterpTime (+ DeltaSeconds (Variables|Default|GetInterpTime)))
  (Transformation|SetActorLocation (Components|GetOwner) (Math|Vector|Lerp(Vector) (CallFunction|GetPointLocation (Variables|Default|GetCurrentPoint)) (CallFunction|GetPointLocation (Variables|Default|GetTargetPoint)) (Math|Curves|GetFloatValue (Variables|Default|GetCurve) (/ (Variables|Default|GetInterpTime) (Variables|Default|GetDuration)))) false false)
  (if (> (Variables|Default|GetInterpTime) (Variables|Default|GetDuration))
    (CallFunction|GetNextPoint)))

(fn SetInitialPosition
  (bind _returnvalue (Components|GetOwner))
  (bind _returnvalue_2 (Components|GetOwner))
  (bind _controlpoints (Variables|Default|GetControlPoints))
  (bind _output (Utilities|Array|Get(acopy) _controlpoints))
  (Utilities|IsValid _returnvalue_2
    (:Is%20Valid
      (Variables|Default|SetActorInitialPosition (Transformation|GetActorLocation _returnvalue_2))
      (if (>= (Utilities|Array|Length (Variables|Default|GetControlPoints)) 2)
        (Utilities|FlowControl|Sequence
          (:then_0
            (if (Variables|Default|GetbPointsAreRelative)
              (Transformation|AddActorLocalOffset _returnvalue _output false true)
              (else
                (Transformation|SetActorLocation _returnvalue _output false true))))
          (:then_1
            (Variables|Default|SetCurrentPoint 0)
            (Variables|Default|SetTargetPoint 1)))
        (else
          (Development|PrintString "Interp Curve Movement needs at least 2 control points."))))))

(fn GetNextPoint
  (bind _controlpoints (Variables|Default|GetControlPoints))
  (bind _returnvalue (Utilities|Array|Length _controlpoints))
  (Variables|Default|SetInterpTime 0.0)
  (if (< (Variables|Default|GetCurrentPoint) (Variables|Default|GetTargetPoint))
    (Math|Integer|IncrementInt (Variables|Default|GetTargetPoint)
      (:%20%20
        (if (>= (Variables|Default|GetTargetPoint) (Utilities|Array|Length (Variables|Default|GetControlPoints)))
          (Variables|Default|SetTargetPoint (- _returnvalue 2))
          (Variables|Default|SetCurrentPoint (- _returnvalue 1))
          (else
            (Math|Integer|IncrementInt (Variables|Default|GetCurrentPoint))))))
    (else
      (bind _result (Math|Integer|DecrementInt (Variables|Default|GetTargetPoint))
        (:%20%20
          (if (<= _result 0)
            (Variables|Default|SetCurrentPoint 0)
            (Variables|Default|SetTargetPoint 1)
            (else
              (Math|Integer|DecrementInt (Variables|Default|GetCurrentPoint)))))))))

(fn GetCurrentPointLocation
  (return (Utilities|Array|Get(acopy) (Variables|Default|GetControlPoints) (Variables|Default|GetCurrentPoint))))

(fn GetPointLocation
  (params (Index :type Integer))
  (if (Variables|Default|GetbPointsAreRelative)
    (return (+ (Utilities|Array|Get(acopy) (Variables|Default|GetControlPoints) Index) (Variables|Default|GetActorInitialPosition)))
    (else
      (return (Utilities|Array|Get(acopy) (Variables|Default|GetControlPoints) Index)))))