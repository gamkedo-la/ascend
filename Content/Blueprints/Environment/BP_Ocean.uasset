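; BP_Ocean is an environment actor that builds an ocean surface from instanced static mesh tiles in its construction script.
; CreateInstances adds one instance when Divisions is zero, otherwise loops over a square grid.
; GetTileLocation spaces tiles by mesh bounds through RemapTileLocation, whose grid-centering formula is left unconnected.
; The event graph has no runtime logic.
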(event EventBeginPlay)

(event Collision|EventActorBeginOverlap
  (params (OtherActor :type Actor%20Object%20Reference)))

(event EventTick
  (params (DeltaSeconds :type Float%20%28single-precision%29)))

(fn ConstructionScript
  (CallFunction|CreateInstances))

(fn CreateInstances
  (bind _divisions (Variables|Default|GetDivisions))
  (bind _instancedstaticmesh (Variables|Default|GetInstancedStaticMesh))
  (if (== (Variables|Default|GetDivisions) 0)
    (Components|InstancedStaticMesh|AddInstance _instancedstaticmesh (Transformation|GetRelativeTransform _instancedstaticmesh) false)
    (else
      (for _index (range 0 _divisions)
        (for _index_2 (range 0 _divisions)
          (Components|InstancedStaticMesh|AddInstance (Variables|Default|GetInstancedStaticMesh) (Math|Transform|MakeTransform (CallFunction|GetTileLocation _index _index_2) "0, 0, 0" "1.000000,1.000000,1.000000") false))))))

(fn GetTileLocation
  (params (x :type Integer) (y :type Integer))
  (bind _instancedstaticmesh (Variables|Default|GetInstancedStaticMesh))
  (bind _staticmesh (Variables|/Script/Engine.StaticMeshComponent|GetStaticMesh _instancedstaticmesh))
  (bind _returnvalue (StaticMesh|GetBounds _staticmesh))
  (bind _returnvalue_2 (* (.boxextent _returnvalue) 2.0))
  (return (Math|Vector|MakeVector (* (Utilities|RemapTileLocation x) (.x _returnvalue_2)) (* (Utilities|RemapTileLocation y) (.y _returnvalue_2)) 0.0)))