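; Procedural actor that builds a tube of Boulder2 meshes along a spline in the Construction Script.
; It samples the spline at constant-velocity intervals set by SplineResolution, calls BuildStructureRing at each and records the local point in SplinePoints.
; Each ring spaces TowerResolution steps around the spline at a fixed radius using rotated forward vectors.
; Every mesh gets its own new InstancedStaticMesh component with a single instance, so instances are not batched.
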(event EventBeginPlay)

(event Collision|EventActorBeginOverlap
  (params (OtherActor :type Actor%20Object%20Reference)))

(event EventTick
  (params (DeltaSeconds :type Float%20%28single-precision%29)))

(fn ConstructionScript
  (bind _splineresolution (Variables|Default|GetSplineResolution))
  (Utilities|Array|Clear (Variables|Default|GetSplinePoints))
  (for _index (range 0 _splineresolution)
    (CallFunction|BuildStructureRing (/ (Math|Conversions|ToFloat(Integer) _index) (Math|Conversions|ToFloat(Integer) _splineresolution)) "/Game/StaticMeshes/Boulders/boulder2.boulder2")
    (Utilities|Array|Add (Variables|Default|GetSplinePoints) (Spline|GetLocationatTime (Variables|Default|GetSpline) (/ (Math|Conversions|ToFloat(Integer) _index) (Math|Conversions|ToFloat(Integer) _splineresolution)) "Local" true))))

(fn BuildStructureRing
  (params (SplinePosition :type Float%20%28double-precision%29) (Mesh :type Static%20Mesh%20Object%20Reference))
  (bind _spline (Variables|Default|GetSpline))
  (bind _returnvalue (Spline|GetTransformatTime _spline SplinePosition "Local" true false))
  (bind (_location _rotation _scale) (Math|Transform|BreakTransform _returnvalue))
  (bind (_roll _pitch _yaw) (Math|Rotator|BreakRotator _rotation))
  (for _index (range 0 (Variables|Default|GetTowerResolution))
    (LocalVariables|SetIndex _index)
    (bind _returnvalue_2 (AddComponent|AddInstancedStaticMeshComponent false))
    (Components|StaticMesh|SetStaticMesh _returnvalue_2 Mesh)
    (Components|InstancedStaticMesh|AddInstance _returnvalue_2 (Math|Transform|MakeTransform (+ _location (* (Math|Vector|GetForwardVector (Math|Rotator|MakeRotator _roll (+ (* (/ 3.6e+02 (Math|Conversions|ToFloat(Integer) (Variables|Default|GetTowerResolution))) (LocalVariables|GetIndex)) _pitch) (+ _yaw 9e+01))) 1000)) _rotation (* _scale 10)) false)))