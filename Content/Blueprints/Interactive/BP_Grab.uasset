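; Grab Blueprint that lets its owning actor pick up and release objects in front of it via the IA_Grab Enhanced Input action.
; On press, FindGrabbies sphere-traces along the owner's forward vector and stores any hit actor implementing BPI_Grabbable as GrabTarget.
; The target attaches to the owner keeping its world position and rotation, without physics handles.
; A DoOnce limits this to one attempt per press; release detaches the target and resets it.
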(event Input|EnhancedActionEvents|EnhancedInputActionIA_Grab
  (params (ActionValue :type Boolean) (ElapsedSeconds :type Float%20%28double-precision%29) (TriggeredSeconds :type Float%20%28double-precision%29) (InputAction :type Input%20Action%20Object%20Reference :default "/Game/ThirdPerson/Input/Actions/IA_Grab.IA_Grab"))
  (bind _grabtarget (Variables|Default|GetGrabTarget))
  (:Triggered
    (Utilities|FlowControl|DoOnce false :!label _label
      (:Completed
        (CallFunction|FindGrabbies)
        (Utilities|IsValid _grabtarget
          (:Is%20Valid
            (Transformation|AttachActorToActor _grabtarget (Components|GetOwner) "None" "KeepWorld" "KeepWorld" "KeepRelative" false))))))
  (:Completed
    (Utilities|IsValid _grabtarget
      (:Is%20Valid
        (Transformation|DetachFromActor _grabtarget "KeepWorld" "KeepWorld" "KeepRelative")
        (goto _label Reset))
      (:Is%20Not%20Valid
        (goto _label Reset)))))

(event EventBeginPlay)

(event EventTick
  (params (DeltaSeconds :type Float%20%28single-precision%29)))

(fn FindGrabbies
  (bind _returnvalue (Components|GetOwner))
  (bind _returnvalue_2 (Transformation|GetActorLocation _returnvalue))
  (Variables|Default|SetGrabTarget 0)
  (bind (_outhit _returnvalue_3) (Collision|SphereTraceByChannel _returnvalue_2 (+ _returnvalue_2 (* (Transformation|GetActorForwardVector _returnvalue) (Variables|Default|GetGrabDistance))) 2e+01 "TraceTypeQuery4" false 0 "None"))
  (if _returnvalue_3
    (Utilities|Casting|CastToBPI_Grabbable (.HitActor (Collision|BreakHitResult _outhit))
      (:then
        (Development|PrintString (Utilities|GetDisplayName (.HitActor (Collision|BreakHitResult _outhit))))
        (Variables|Default|SetGrabTarget (.HitActor (Collision|BreakHitResult _outhit)))
        (return true))
      (:CastFailed
        _)))
  (return false))