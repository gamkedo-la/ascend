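; BP_Cube is a physics cube that can be levitated toward a referenced actor and released.
; LevitateCube, gated by two flags set through CanLevitate and LaunchCube, disables physics simulation and sets collision to physics-only.
; Each call lerps the cube toward a fixed world-space offset from that actor, so smooth following relies on repeated calls.
; ReleaseCube restores physics and full collision; LaunchCube applies no force.
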(event EventReleaseCube
  (bind _staticmesh (Variables|Default|GetStaticMesh))
  (Physics|SetSimulatePhysics _staticmesh true)
  (Collision|SetCollisionEnabled _staticmesh "QueryAndPhysics"))

(event EventLevitateCube
  (params (PREF :type Actor%20Object%20Reference))
  (bind _staticmesh (Variables|Default|GetStaticMesh))
  ;[1 1 1] Event Levitate
  (if (Variables|Default|GetCan%20Levitate)
    (if (Variables|Default|GetCan%20Levitate%20After)
      (CallFunction|Levitate PREF)
      (Physics|SetSimulatePhysics _staticmesh false)
      (Collision|SetCollisionEnabled _staticmesh "PhysicsOnly"))))

(event EventCanLevitate
  (params (CanLevitate :type Boolean))
  ;[1 1 1] Event Can Levitate
  (Variables|Default|SetCan%20Levitate CanLevitate))

(event EventLaunchCube
  (params (LaunchAlph :type Float%20%28double-precision%29) (CanLevitateAfter :type Boolean))
  ;[1 1 1] Event Launch Cube
  (Variables|Default|SetCan%20Levitate%20After CanLevitateAfter))

(fn ConstructionScript)

(fn Levitate
  (params (PREF :type Actor%20Object%20Reference))
  (Variables|Default|SetPREF PREF)
  (Transformation|SetActorLocation (Math|Vector|Lerp(Vector) (Transformation|GetActorLocation self) (+ (+ (Transformation|GetActorLocation (Variables|Default|GetPREF)) "0.000000,350.000000,150.000000") (* (Transformation|GetActorRightVector (Variables|Default|GetPREF)) 0.0)) 0.08) false false))