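; Procedural mesh Blueprint that builds a lathe-style surface of revolution around the Z axis, entirely in the Construction Script.
; Constrained handles shape it: HeightHandle sets total height, and each RingCenters entry's X sets the radius of an evenly spaced ring.
; Rings are swept by yaw at the set Resolution, then given scaled UVs and grid triangles.
; The resulting section gets calculated normals and tangents, collision and a material.
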(event EventBeginPlay)

(event Collision|EventActorBeginOverlap
  (params (OtherActor :type Actor%20Object%20Reference)))

(event EventTick
  (params (DeltaSeconds :type Float%20%28single-precision%29)))

(fn ConstructionScript
  (bind _uvs (Variables|Default|GetUVs))
  (bind _outposition (CallFunction|ConstrainHandleZ (Variables|Default|GetHeightHandle) "-100.000000,0.000000,0.000000"))
  (Variables|Default|SetHeightHandle _outposition)
  (CallFunction|SetHandlePositions)
  (CallFunction|BuildVertexPositions)
  (CallFunction|MakeUVs)
  (CallFunction|CreateTriangles)
  (bind (_normals _tangents) (Class|KismetProceduralMeshLibrary|CalculateTangentsforMesh (Variables|Default|GetVertexPositions) (Variables|Default|GetTriangles) (Variables|Default|GetUVs)))
  (Class|ProceduralMeshComponent|CreateMeshSectionLinearColor (Variables|Default|GetProceduralMesh) 0 (Variables|Default|GetVertexPositions) (Variables|Default|GetTriangles) _normals _uvs _uvs _uvs _uvs 0 _tangents true false)
  (Rendering|Material|SetMaterial (Variables|Default|GetProceduralMesh) 0 (Variables|Default|GetMaterial)))

(fn ConstrainHandleX
  (params (InPosition :type Vector) (Offset :type Vector))
  (bind _output_get (LocalVariables|SetTempHandle InPosition))
  (return (+ (Math|Vector|MakeVector (Math|Float|Clamp(Float) (.X (Math|Vector|BreakVector _output_get)) 0.0 1e+05) 0.0 0.0) Offset)))

(fn ConstrainHandleZ
  (params (InPosition :type Vector) (Offset :type Vector))
  (bind _output_get (LocalVariables|SetTempHandle InPosition))
  (return (+ (Math|Vector|MakeVector 0.0 0.0 (Math|Float|Clamp(Float) (.Z (Math|Vector|BreakVector _output_get)) 0.0 1e+05)) Offset)))

(fn SetHandlePositions
  (for (_array_element _array_index) (Variables|Default|GetRingCenters)
    (bind _outposition (CallFunction|ConstrainHandleX (Math|Vector|MakeVector (.X (Math|Vector|BreakVector _array_element)) (.Y (Math|Vector|BreakVector _array_element)) 0.0) (Math|Vector|MakeVector 0.0 0.0 (* _array_index (.Z (Math|Vector|BreakVector (/ (Variables|Default|GetHeightHandle) (- (Utilities|Array|Length (Variables|Default|GetRingCenters)) 1))))))))
    (Utilities|Array|SetArrayElem (Variables|Default|GetRingCenters) _array_index _outposition true)))

(fn BuildVertexPositions
  (bind _resolution (Variables|Default|GetResolution))
  (Utilities|Array|Clear (Variables|Default|GetVertexPositions))
  (for _array_element (Variables|Default|GetRingCenters)
    (LocalVariables|SetRingCenter _array_element)
    (for _index (range 0 _resolution)
      (Utilities|Array|Add (Variables|Default|GetVertexPositions) (+ (+ (* (Math|Vector|GetForwardVector (Math|Rotator|MakeRotator 0.0 0.0 (Math|Conversions|ToFloat(Integer) (* _index (/ 360 _resolution))))) (.X (Math|Vector|BreakVector (LocalVariables|GetRingCenter)))) "") (Math|Vector|MakeVector 0.0 0.0 (.Z (Math|Vector|BreakVector (LocalVariables|GetRingCenter))))))))
  (for _array_element_2 (Variables|Default|GetVertexPositions)
    _))

(fn MakeUVs
  (bind _uvscale (Variables|Default|GetUVScale))
  (Utilities|Array|Clear (Variables|Default|GetUVs))
  (for _index (range 0 (- (Utilities|Array|Length (Variables|Default|GetRingCenters)) 1))
    (LocalVariables|SetZ _index)
    (for _index_2 (range 0 (Variables|Default|GetResolution))
      (LocalVariables|SetX _index_2)
      (Utilities|Array|Add (Variables|Default|GetUVs) (Math|Vector2D|MakeVector2D (* (/ (LocalVariables|GetX) (Variables|Default|GetResolution)) (.x _uvscale)) (* (.y _uvscale) (/ (LocalVariables|GetZ) (Utilities|Array|Length (Variables|Default|GetRingCenters)))))))))

(fn CreateTriangles
  (Utilities|Array|Clear (Variables|Default|GetTriangles))
  (bind _triangles (Class|KismetProceduralMeshLibrary|CreateGridMeshTriangles (+ (Utilities|Array|Length (Variables|Default|GetRingCenters)) 0) (+ (Variables|Default|GetResolution) 1) true))
  (Variables|Default|SetTriangles _triangles))